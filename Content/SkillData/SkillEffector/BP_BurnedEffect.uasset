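; Burn status effect actor that tints and damages its owning character for a few seconds.
; On BeginPlay, if the owner implements ICharacter, it tints the body dark red through an interface message and starts a looping timer applying DamageType_Dot damage each second.
; After a short delay it resets the color and destroys itself.
; Owners without the interface get no effect, and the actor does not self-destroy.
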(event Custom|커스텀이벤트_0
  (Game|Damage|ApplyDamage (Components|GetOwner) 3.0 0 self "/Game/DamageType/DamageType_Dot.DamageType_Dot_C"))

(event EventBeginPlay
  (bind _returnvalue (Components|GetOwner))
  (if (Utilities|DoesObjectImplementInterface _returnvalue "/Script/Magician.ICharacter")
    (Class|ICharacter|ChangeBodyColor(Message) _returnvalue "(R=0.200000,G=0.019608,B=0.047059,A=1.000000)" 1e+01)
    (Utilities|Time|SetTimerbyEvent (delegate Custom|커스텀이벤트_0) 1.0 true)
    (Utilities|FlowControl|Delay 3.0)
    (Class|ICharacter|ChangeBodyColor(Message) _returnvalue "(R=1.000000,G=1.000000,B=1.000000,A=1.000000)" 0.0)
    (Actor|DestroyActor)))

(fn ConstructionScript)