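; BP_FrozenEffect is a skill effector actor that applies a timed freeze visual to its owner.
; On BeginPlay, if the owner implements ICharacter, it tints the body blue via an interface message, waits five seconds, restores the color and destroys itself.
; StopMovement is a stub called at both ends: it casts to Character and only prints Stop or Go, so movement is unaffected.
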(event EventBeginPlay
  (bind _returnvalue (Components|GetOwner))
  (if (Utilities|DoesObjectImplementInterface _returnvalue "/Script/Magician.ICharacter")
    (Class|ICharacter|ChangeBodyColor(Message) _returnvalue "(R=0.128734,G=0.156389,B=0.635417,A=1.000000)" 1e+01)
    (CallFunction|StopMovement _returnvalue true)
    (Utilities|FlowControl|Delay 5.0)
    (Class|ICharacter|ChangeBodyColor(Message) _returnvalue "(R=1.000000,G=1.000000,B=1.000000,A=1.000000)" 0.0)
    (CallFunction|StopMovement _returnvalue false)
    (Actor|DestroyActor)))

(fn ConstructionScript)

(fn StopMovement
  (params (InActor :type Actor%20Object%20Reference) (bStop :type Boolean))
  (bind _ascharacter (Utilities|Casting|CastToCharacter InActor))
  (LocalVariables|SetInChar _ascharacter)
  (if bStop
    (Development|PrintString "Stop")
    (else
      (Development|PrintString "Go"))))