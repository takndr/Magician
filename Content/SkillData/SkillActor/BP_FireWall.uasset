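; BP_FireWall is a skill actor that raises a three-stage fire effect from its owner's transform, lowered toward the ground.
; On BeginPlay, SetAttack activates three particle and collision box pairs in a timed sequence, each using SkillEffect.
; Overlapped CEnemy actors are recorded in HittedActor, which the later two boxes check to skip repeat hits.
; SkillDamage is only printed, not applied.
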(event OnComponentBeginOverlap(Box)
  (params (OverlappedComponent :type Primitive%20Component%20Object%20Reference) (OtherActor :type Actor%20Object%20Reference) (OtherComp :type Primitive%20Component%20Object%20Reference) (OtherBodyIndex :type Integer) (bFromSweep :type Boolean) (SweepResult :type Hit%20Result%20Structure%20%28by%20ref%29))
  (if (!= OtherActor (Components|GetOwner))
    (bind _ascenemy (Utilities|Casting|CastToCEnemy OtherActor))
    (Utilities|Array|AddUnique (Variables|Default|GetHittedActor) _ascenemy)
    (Development|PrintString (Utilities|String|ToString(Float) (Variables|/Script/Magician.CSkillData|GetSkillDamage (Variables|Default|GetSkillData))))))

(event OnComponentBeginOverlap(Box1)
  (params (OverlappedComponent :type Primitive%20Component%20Object%20Reference) (OtherActor :type Actor%20Object%20Reference) (OtherComp :type Primitive%20Component%20Object%20Reference) (OtherBodyIndex :type Integer) (bFromSweep :type Boolean) (SweepResult :type Hit%20Result%20Structure%20%28by%20ref%29))
  (if (!= OtherActor (Components|GetOwner))
    (if (== (Utilities|Array|FindItem (Variables|Default|GetHittedActor) OtherActor) -1)
      (bind _ascenemy (Utilities|Casting|CastToCEnemy OtherActor))
      (Utilities|Array|AddUnique (Variables|Default|GetHittedActor) _ascenemy)
      (Development|PrintString (Utilities|String|ToString(Float) (Variables|/Script/Magician.CSkillData|GetSkillDamage (Variables|Default|GetSkillData))))
      (else
        (Development|PrintString "Already Hitted")))))

(event OnComponentBeginOverlap(Box2)
  (params (OverlappedComponent :type Primitive%20Component%20Object%20Reference) (OtherActor :type Actor%20Object%20Reference) (OtherComp :type Primitive%20Component%20Object%20Reference) (OtherBodyIndex :type Integer) (bFromSweep :type Boolean) (SweepResult :type Hit%20Result%20Structure%20%28by%20ref%29))
  (if (!= OtherActor (Components|GetOwner))
    (if (== (Utilities|Array|FindItem (Variables|Default|GetHittedActor) OtherActor) -1)
      (bind _ascenemy (Utilities|Casting|CastToCEnemy OtherActor))
      (Utilities|Array|AddUnique (Variables|Default|GetHittedActor) _ascenemy)
      (Development|PrintString (Utilities|String|ToString(Float) (Variables|/Script/Magician.CSkillData|GetSkillDamage (Variables|Default|GetSkillData))))
      (else
        (Development|PrintString "Already Hitted")))))

(event EventBeginPlay
  (CallFunction|SetTransform)
  (CallFunction|SetAttack (Variables|Default|GetParticleSystem) (Variables|Default|GetBox))
  (Utilities|FlowControl|Delay 0.3)
  (CallFunction|SetAttack (Variables|Default|GetParticleSystem1) (Variables|Default|GetBox1))
  (Utilities|FlowControl|Delay 0.3)
  (CallFunction|SetAttack (Variables|Default|GetParticleSystem2) (Variables|Default|GetBox2)))

(event Collision|EventActorBeginOverlap
  (params (OtherActor :type Actor%20Object%20Reference)))

(fn ConstructionScript)

(fn SetAttack
  (params (Particle :type Particle%20System%20Component%20Object%20Reference) (Collision :type Box%20Component%20Object%20Reference))
  (Effects|Components|ParticleSystem|SetTemplate Particle (Variables|Default|GetSkillEffect))
  (Collision|SetCollisionEnabled Collision "QueryAndPhysics"))

(fn SetTransform
  (bind _returnvalue (Components|GetOwner))
  (bind _returnvalue_2 (Components|GetOwner))
  (bind _returnvalue_3 (Transformation|GetActorTransform _returnvalue))
  (bind _returnvalue_4 (Transformation|GetActorLocation _returnvalue_2))
  (Transformation|SetActorTransform (Math|Transform|MakeTransform (Math|Vector|MakeVector (.x _returnvalue_4) (.y _returnvalue_4) (- (.z _returnvalue_4) 88.0)) (.rotation _returnvalue_3) (.scale _returnvalue_3))))