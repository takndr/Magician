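; BP_FireBall is a fireball skill projectile launched from its owning actor.
; On BeginPlay it snaps to just in front of the owner with matching rotation and scale, applies the SkillEffect particle template, and fires along the owner's forward vector.
; Overlapping any actor other than the owner spawns the HitEffect and destroys it, with SkillDamage only printed as a string, not applied.
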(event EventBeginPlay
  (bind _projectilemovement (Variables|Default|GetProjectileMovement))
  (CallFunction|SetTransform)
  (Effects|Components|ParticleSystem|SetTemplate (Variables|Default|GetParticleSystem) (Variables|Default|GetSkillEffect))
  (Variables|/Script/Engine.MovementComponent|SetVelocity _projectilemovement (* (Transformation|GetActorForwardVector (Components|GetOwner)) (Variables|/Script/Engine.ProjectileMovementComponent|GetInitialSpeed _projectilemovement))))

(event Collision|EventActorBeginOverlap
  (params (OtherActor :type Actor%20Object%20Reference))
  (if (!= OtherActor (Components|GetOwner))
    (Effects|SpawnEmitteratLocation (Variables|Default|GetHitEffect) (Transformation|GetActorLocation))
    (Development|PrintString (Utilities|String|ToString(Float) (Variables|Default|GetSkillDamage)))
    (Actor|DestroyActor)))

(fn ConstructionScript)

(fn SetTransform
  (bind _returnvalue (Components|GetOwner))
  (bind _returnvalue_2 (Components|GetOwner))
  (bind _returnvalue_3 (Transformation|GetActorTransform _returnvalue))
  (Transformation|SetActorTransform (Math|Transform|MakeTransform (+ (Transformation|GetActorLocation _returnvalue_2) (* (Transformation|GetActorForwardVector _returnvalue_2) 5e+01)) (.rotation _returnvalue_3) (.scale _returnvalue_3))))