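; BP_FireWall is a fire wall skill effect actor that ignites in three staggered segments when spawned.
; BeginPlay calls SetAttack on three particle and box collision pairs in sequence, separated by short delays.
; SetAttack assigns the SkillEffect template to the particle system and turns on overlap events for its box.
; The overlap and Tick events are empty, so no damage logic appears in this graph.
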(event EventBeginPlay
  (CallFunction|SetAttack (Variables|Default|GetParticleSystem) (Variables|Default|GetBox))
  (Utilities|FlowControl|Delay 0.3)
  (CallFunction|SetAttack (Variables|Default|GetParticleSystem1) (Variables|Default|GetBox1))
  (Utilities|FlowControl|Delay 0.3)
  (CallFunction|SetAttack (Variables|Default|GetParticleSystem2) (Variables|Default|GetBox2)))

(event Collision|EventActorBeginOverlap
  (params (OtherActor :type Actor%20Object%20Reference)))

(event EventTick
  (params (DeltaSeconds :type Float%20%28single-precision%29)))

(fn ConstructionScript)

(fn SetAttack
  (params (Particle :type Particle%20System%20Component%20Object%20Reference) (Collision :type Box%20Component%20Object%20Reference))
  (Effects|Components|ParticleSystem|SetTemplate Particle (Variables|Default|GetSkillEffect))
  (Variables|/Script/Engine.PrimitiveComponent|SetbGenerateOverlapEvents Collision true))