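; Ice wall skill effect actor built around a Niagara system.
; On BeginPlay it copies its owner's location, rotation and scale, lowering the location by a fixed Z offset.
; It then registers itself as the Niagara "CallBack" object variable.
; The ParticleData event is only a stub that prints a debug string.
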(event EventBeginPlay
  (CallFunction|SetTransform)
  (Class|NiagaraComponent|SetVariableObject (Variables|Default|GetNiagara) "CallBack" self))

(event EventParticleData
  (params (Data :type Array%20of%20Basic%20Particle%20Data%20Structures) (NiagaraSystem :type Niagara%20System%20Object%20Reference))
  (Development|PrintString "Hello"))

(fn ConstructionScript)

(fn SetTransform
  (bind _returnvalue (Components|GetOwner))
  (bind _returnvalue_2 (Components|GetOwner))
  (bind _returnvalue_3 (Transformation|GetActorTransform _returnvalue))
  (bind _returnvalue_4 (Transformation|GetActorLocation _returnvalue_2))
  (Transformation|SetActorTransform (Math|Transform|MakeTransform (Math|Vector|MakeVector (.x _returnvalue_4) (.y _returnvalue_4) (- (.z _returnvalue_4) 88.0)) (.rotation _returnvalue_3) (.scale _returnvalue_3))))